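; Enemy actor that bobs its body vertically on a Timeline, turns to face the player and fires hitscan shots.
; Pawn sensing starts rotation and a DoOnce-guarded looping fire timer, both stopped by a retriggerable delay once sightings cease.
; Each shot line-traces forward with random upward spread, applies damage and briefly swaps Niagara effects.
; Incoming damage reduces health, playing a hurt sound or destroying the enemy.
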(event OnSeePawn(PawnSensing)
  (params (Pawn :type Pawn%20Object%20Reference))
  ;[1 1 1] Looking at Player
  (Variables|Default|SetShouldRotate? true)
  (CallFunction|ShootPlayer)
  (Utilities|FlowControl|RetriggerableDelay 4.0)
  (Variables|Default|SetShouldRotate? false)
  (Utilities|Time|ClearandInvalidateTimerbyHandle (Variables|Default|GetShootEvent))
  (CallFunction|ResetDoOnce))

(event Custom|ShootPlayer
  (Utilities|FlowControl|DoOnce false
    (:Completed
      (bind _returnvalue (Utilities|Time|SetTimerbyEvent (delegate Custom|Shoot) (Variables|Default|GetFirerate) true))
      (Variables|Default|SetShootEvent _returnvalue))))

(event Custom|Shoot
  (bind _returnvalue (Transformation|GetActorLocation))
  (Audio|PlaySoundatLocation "/Game/Kenny/Kenny/sounds/enemy_attack.enemy_attack" _returnvalue "0, 0, 0" 1.0 1.0 0.0 0 0 0 0)
  (bind _outhit (Collision|LineTraceByChannel _returnvalue (+ (+ _returnvalue (* (Math|Vector|GetForwardVector (Transformation|GetActorRotation)) (Variables|Default|GetFireDistance))) (Math|Vector|MakeVector 0.0 0.0 (Math|Random|RandomFloatinRange 0.0 5e+02))) "TraceTypeQuery1" false 0 "None"))
  (Game|Damage|ApplyDamage (.HitActor (Collision|BreakHitResult _outhit)) 1.0 0 0)
  (Class|NiagaraComponent|SetAsset (Variables|Default|Getparticle) "/Game/Particles/NS_Enemy1.NS_Enemy1" true)
  (Utilities|FlowControl|Delay 0.2)
  (Class|NiagaraComponent|SetAsset (Variables|Default|Getparticle) "/Game/Particles/NS_Enemy2.NS_Enemy2" true))

(event Custom|ResetDo%20once
  (Utilities|FlowControl|DoOnce false) ; enters at Reset
)

(event EventBeginPlay
  (bind _enemybody (Variables|Default|GetEnemyBody))
  (bind _relativelocation (Variables|/Script/Engine.SceneComponent|GetRelativeLocation _enemybody))
  ;[1 1 1] Enemy Movement
  (bind _enemymovement (Timeline|Timeline Play)
    (:Update
      (Transformation|SetRelativeLocation _enemybody (Math|Vector|MakeVector (.x _relativelocation) (.y _relativelocation) (Math|Float|Lerp 0.0 (Variables|Default|GetEnemyMovementDistance) _enemymovement)) false false))))

(event Collision|EventActorBeginOverlap
  (params (OtherActor :type Actor%20Object%20Reference)))

(event EventTick
  (params (DeltaSeconds :type Float%20%28single-precision%29))
  ;[1 1 1] Looking at Player
  (if (Variables|Default|GetShouldRotate?)
    (Transformation|SetActorRotation (Math|Rotator|FindLookatRotation (Transformation|GetActorLocation) (Transformation|GetActorLocation (Game|GetPlayerCharacter 0))))))

(event Game|Damage|EventAnyDamage
  (params (Damage :type Float%20%28single-precision%29) (DamageType :type Damage%20Type%20Object%20Reference) (InstigatedBy :type Controller%20Object%20Reference) (DamageCauser :type Actor%20Object%20Reference))
  (bind _output_get (Variables|Default|SetHealth (- (Variables|Default|GetHealth) Damage)))
  (if (<= _output_get 0.0)
    (Audio|PlaySoundatLocation "/Game/Kenny/Kenny/sounds/enemy_destroy.enemy_destroy" (Transformation|GetActorLocation) "0, 0, 0" 1.0 1.0 0.0 0 0 0 0)
    (Actor|DestroyActor)
    (else
      (Audio|PlaySoundatLocation "/Game/Kenny/Kenny/sounds/enemy_hurt.enemy_hurt" (Transformation|GetActorLocation) "0, 0, 0" 1.0 1.0 0.0 0 0 0 0))))

(fn ConstructionScript)